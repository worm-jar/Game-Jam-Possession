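; PlatformToMove is a Blueprint that moves a museum grillage mesh along a spline when GateFunction is triggered.
; A timeline, with play rate set from Speed at BeginPlay, drives a lerp over the spline length to set the mesh's world location.
; A DoOnce adds an audio component on the first update, then the timeline's finish stops that sound and resets the DoOnce.
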(event `self.ReceiveBeginPlay`
  (set `self.LocationStart` (`SceneComponent.K2_GetComponentLocation` (`self.PROP_Museum_Grillage`)))
  (`TimelineComponent.SetPlayRate` (`self.Timeline`) (`self.Speed`)))

(event `self.GateFunction`
  (bind (_direction _newtrack_0) (`Timeline|Timeline`)
    (:`Update`
      (bind _returnvalue_location (`KismetMathLibrary.BreakTransform` (`SplineComponent.GetTransformAtDistanceAlongSpline` (`self.Spline`) (`KismetMathLibrary.Lerp` 0.0 (`SplineComponent.GetSplineLength` (`self.Spline`)) _newtrack_0) "World" false)))
      (`SceneComponent.K2_SetWorldTransform` (`self.PROP_Museum_Grillage`) (`KismetMathLibrary.MakeTransform` _returnvalue_location) false false)
      (`/Engine/EditorBlueprintResources/StandardMacros.DoOnce` false :!label _label
        (:`Completed`
          (bind _returnvalue (`AddComponent|NODE_AddAudioComponent-1`))
          (set `self.RefSound` _returnvalue))))
    (:`Finished`
      (`AudioComponent.Stop` (`self.RefSound`))
      (goto _label :!via `Reset`))))

(fn `UserConstructionScript`)
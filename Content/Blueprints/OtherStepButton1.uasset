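; A pressure button actor that sinks when a possessable actor steps on it and notifies a linked gate.
; BeginPlay caches the button mesh's world position, and any overlap on the trigger box plays a button sound.
; A DoOnce then lets only the first overlap through, which, if tagged Possessable, lowers the button and calls GateFunctionMessage on MoveRef.
; The DoOnce is never reset, so an untagged first overlap uses it up.
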(event `self.ReceiveBeginPlay`
  (set `self.NewVar` (`SceneComponent.K2_GetComponentLocation` (`self.Button`))))

(event `self.Box.OnComponentBeginOverlap`
  (params (OverlappedComponent :type "PrimitiveComponent Object Reference") (OtherActor :type "Actor Object Reference") (OtherComp :type "PrimitiveComponent Object Reference") (OtherBodyIndex :type Integer) (bFromSweep :type Boolean) (SweepResult :type "HitResult Structure (by ref)"))
  (`GameplayStatics.PlaySound2D` "/Game/SFX/Buttons.Buttons" 1.0 1.0 0.0 null null)
  (`/Engine/EditorBlueprintResources/StandardMacros.DoOnce` false
    (:`Completed`
      (if (`self.ActorHasTag` OtherActor "Possessable")
        (`SceneComponent.K2_SetWorldLocation` (`self.Button`) (- (`self.NewVar`) (0.0 0.0 13.0)) false false)
        (message `/Game/Blueprints/Interfaces/GateMoveInterface.GateFunction` (`self.MoveRef`))))))

(fn `UserConstructionScript`)
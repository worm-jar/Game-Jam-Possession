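; Pressable button actor that triggers either a linked cube's interaction or a linked door's rotation.
; Press plays a sound, nudges the cylinder mesh downward, then calls Interact on CubeRef if it has the "cube" tag, otherwise Rotate on DoorToRotate.
; A DoOnce gate blocks repeat presses until a short delay restores the cylinder to its location saved at BeginPlay.
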(event `self.ReceiveBeginPlay`
  (set `self.InitLoc` (`SceneComponent.K2_GetComponentLocation` (`self.Cylinder`))))

(event `/Game/Blueprints/Interfaces/PlayerToButtonWall.Press`
  (`/Engine/EditorBlueprintResources/StandardMacros.DoOnce` false :!label _label
    (:`Completed`
      (`GameplayStatics.PlaySound2D` "/Game/SFX/Buttons.Buttons" 1.0 1.0 0.0 null null)
      (`SceneComponent.K2_AddLocalOffset` (`self.Cylinder`) (* (`KismetMathLibrary.Normal` (`KismetMathLibrary.Vector_Down`)) (10.0 10.0 10.0)) false false)
      (if (`self.ActorHasTag` (`self.CubeRef`) "cube")
        (`/Game/Blueprints/CubeToMove.Interact` (`self.CubeRef`))
        (else
          (`/Game/Blueprints/Door.Rotate` (`self.Door to Rotate`))))
      (`KismetSystemLibrary.Delay` 1.8)
      (`SceneComponent.K2_SetWorldLocation` (`self.Cylinder`) (`self.InitLoc`) false false)
      (goto _label :!via `Reset`))))

(fn `UserConstructionScript`)
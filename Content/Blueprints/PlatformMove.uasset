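; Moving platform actor that carries its Platform component along the FollowSpline path.
; On BeginPlay, it sets the timeline's play rate from Speed and plays it.
; Each update maps the timeline track onto the spline's length and sets the platform's world transform from that point, taking only the location from the spline.
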(event `self.ReceiveBeginPlay`
  (`TimelineComponent.SetPlayRate` (`self.Timeline`) (`self.Speed`))
  (bind (_direction _newtrack_0) (`Timeline|Timeline`)
    (:`Update`
      (bind _returnvalue_location (`KismetMathLibrary.BreakTransform` (`SplineComponent.GetTransformAtDistanceAlongSpline` (`self.FollowSpline`) (`KismetMathLibrary.Lerp` 0.0 (`SplineComponent.GetSplineLength` (`self.FollowSpline`)) _newtrack_0) "World" false)))
      (`SceneComponent.K2_SetWorldTransform` (`self.Platform`) (`KismetMathLibrary.MakeTransform` _returnvalue_location) false false))))

(fn `UserConstructionScript`)
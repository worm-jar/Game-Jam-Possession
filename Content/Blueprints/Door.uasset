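; Door actor that swings its static mesh open and closed through Rotate and UnRotate events.
; A timeline drives a rotation lerp between the world rotations of the Start and End components, and UnRotate reverses it.
; The timeline update also passes through a DoOnce that is never reset, so the 2D opening sound plays only the first time.
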(event `/Game/Blueprints/Interfaces/InteractDoorInterface.Rotate`
  (bind (_direction _newtrack_0) (`Timeline|Timeline` :!label _label)
    (:`Update`
      (`SceneComponent.K2_SetWorldRotation` (`self.StaticMesh`) (`KismetMathLibrary.RLerp` (`SceneComponent.K2_GetComponentRotation` (`self.Start`)) (`SceneComponent.K2_GetComponentRotation` (`self.End`)) _newtrack_0) false false)
      (`/Engine/EditorBlueprintResources/StandardMacros.DoOnce` false
        (:`Completed`
          (`GameplayStatics.PlaySound2D` "/Game/SFX/Open_Door.Open_Door" 10.0 1.0 0.0 null null))))))

(event `/Game/Blueprints/Interfaces/InteractDoorInterface.UnRotate`
  (goto _label :!via `Reverse`))

(fn `UserConstructionScript`)
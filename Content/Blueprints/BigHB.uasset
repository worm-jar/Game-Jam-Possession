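; BigHB is a pressure button that reacts to actors tagged Possessable overlapping its Box.
; On such an overlap it sinks the Button, calls Interact on CubeRef and rotates DoorToRotate; end overlap restores the Button and calls Return on CubeRef, leaving the door untouched.
; Any overlap begin or end plays a sound.
; A DoOnce resets only after a tagged press, so an untagged overlap blocks later presses.
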(event `self.ReceiveBeginPlay`
  (set `self.NewVar` (`SceneComponent.K2_GetComponentLocation` (`self.Button`))))

(event `self.Box.OnComponentBeginOverlap`
  (params (OverlappedComponent :type "PrimitiveComponent Object Reference") (OtherActor :type "Actor Object Reference") (OtherComp :type "PrimitiveComponent Object Reference") (OtherBodyIndex :type Integer) (bFromSweep :type Boolean) (SweepResult :type "HitResult Structure (by ref)"))
  (`GameplayStatics.PlaySound2D` "/Game/SFX/Buttons.Buttons" 1.0 1.0 0.0 null null)
  (`/Engine/EditorBlueprintResources/StandardMacros.DoOnce` false :!label _label
    (:`Completed`
      (if (`self.ActorHasTag` OtherActor "Possessable")
        (`SceneComponent.K2_SetWorldLocation` (`self.Button`) (- (`self.NewVar`) (0.0 0.0 13.0)) false false)
        (`/Game/Blueprints/CubeToMove.Interact` (`self.CubeRef`))
        (`/Game/Blueprints/Door.Rotate` (`self.Door to Rotate`))
        (goto _label :!via `Reset`)))))

(event `self.Box.OnComponentEndOverlap`
  (params (OverlappedComponent :type "PrimitiveComponent Object Reference") (OtherActor :type "Actor Object Reference") (OtherComp :type "PrimitiveComponent Object Reference") (OtherBodyIndex :type Integer))
  (`GameplayStatics.PlaySound2D` "/Game/SFX/Buttons.Buttons" 1.0 1.0 0.0 null null)
  (if (`self.ActorHasTag` OtherActor "Possessable")
    (`SceneComponent.K2_SetWorldLocation` (`self.Button`) (`self.NewVar`) false false)
    (`/Game/Blueprints/CubeToMove.Return` (`self.CubeRef`))))

(fn `UserConstructionScript`)
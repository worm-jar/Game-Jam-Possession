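; BreakableCube is an actor in the DO_NOT_USE folder that breaks into a SmallCloth actor.
; Its Breaking event spawns SmallCloth at the Breakable component's world location, then destroys the cube.
; An unconnected branch, commented as useless, holds life-counter logic that would swap to a broken material before destruction.
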(event `Breaking`
  (`|SpawnActorFromClass` "/Game/Blueprints/SmallCloth.SmallCloth_C" (`KismetMathLibrary.MakeTransform` (`SceneComponent.K2_GetComponentLocation` (`self.Breakable`))) "Undefined" "MultiplyWithRoot" null null)
  (`self.K2_DestroyActor`))

(fn `UserConstructionScript`)
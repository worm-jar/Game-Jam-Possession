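; BigCloth is an actor that pairs a large skeletal mesh cloth with a BreakableCube child actor.
; On BeginPlay it casts the child actor to BreakableCube and hands it a reference to the cloth through NewVar.
; Its Breaking event, not called within this Blueprint, destroys every SkeletalMeshActor in the level rather than targeting its own cloth.
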(event `self.ReceiveBeginPlay`
  (bind _asbreakable_cube (cast `/Game/Blueprints/DO_NOT_USE/BreakableCube` (`ChildActorComponent.ChildActor` (`self.BreakableCube`))))
  (set `/Game/Blueprints/DO_NOT_USE/BreakableCube.NewVar` (`self.SKM_BLKT_Toile_Full_2x6_HighPoly`) _asbreakable_cube))

(event `Breaking`
  (bind _outactors (`GameplayStatics.GetAllActorsOfClass` "/Script/Engine.SkeletalMeshActor"))
  (for _array_element _outactors
    (`self.K2_DestroyActor` _array_element)))

(fn `UserConstructionScript`)